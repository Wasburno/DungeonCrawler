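; BP_Sword is a melee weapon that damages BP_BasicEnemy actors it overlaps while triggered.
; Its damage collision starts disabled, and Tick switches it between query-only and no collision according to the MIsTriggered flag.
; On begin overlap, it casts the other actor to BP_BasicEnemy, applies MDamage unless that enemy is invulnerable, and prints the enemy's HP.
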(event `self.ReceiveBeginPlay`
  (`PrimitiveComponent.SetCollisionEnabled` (`self.m_damageCollision`) "NoCollision"))

(event `self.ReceiveTick`
  (params (DeltaSeconds :type "Float (single-precision)"))
  (if (`self.m_isTriggered`)
    (`PrimitiveComponent.SetCollisionEnabled` (`self.m_damageCollision`) "QueryOnly")
    (else
      (`PrimitiveComponent.SetCollisionEnabled` (`self.m_damageCollision`) "NoCollision"))))

(event `self.m_damageCollision.OnComponentBeginOverlap`
  (params (OverlappedComponent :type "PrimitiveComponent Object Reference") (OtherActor :type "Actor Object Reference") (OtherComp :type "PrimitiveComponent Object Reference") (OtherBodyIndex :type Integer) (bFromSweep :type Boolean) (SweepResult :type "HitResult Structure (by ref)"))
  (bind _asbp_basic_enemy (cast `/Game/Blueprints/BP_BasicEnemy` OtherActor))
  (if (not (`/Game/Blueprints/BP_BasicEnemy.isInvulnerable` _asbp_basic_enemy))
    (`/Game/Blueprints/BP_BasicEnemy.takeDamage` _asbp_basic_enemy (`self.m_damage`))
    (`KismetSystemLibrary.PrintString` (`KismetStringLibrary.Conv_DoubleToString` (`/Game/Blueprints/BP_BasicEnemy.hp` _asbp_basic_enemy)))))

(fn `UserConstructionScript`)