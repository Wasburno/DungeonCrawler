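; BP_BasicEnemy is a melee enemy that chases the player once its pawn sensing spots a pawn.
; On reaching the player it plays an attack montage and, after a delay, enables a hand-socketed sphere that damages a non-invulnerable player on overlap.
; TakeDamage grants timed invulnerability counted down on Tick, or at zero HP disables capsule collision and adds a kill.
; Delayed destruction runs only when FollowTarget fires again from a sighting after death.
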(event `self.ReceiveBeginPlay`
  (`SceneComponent.K2_AttachToComponent` (`self.Sphere`) (`self.Mesh`) "RHSocket" "KeepRelative" "KeepRelative" "KeepRelative" true)
  (`PrimitiveComponent.SetCollisionEnabled` (`self.Sphere`) "NoCollision")
  (set `self.canAttack` true)
  (set `self.canMove` true)
  (set `self.hp` (`self.hpBase`)))

(event `self.ReceiveTick`
  (params (DeltaSeconds :type "Float (single-precision)"))
  (`self.checkInvulnerability`))

(event `self.PawnSensing.OnSeePawn`
  (params (Pawn :type "Pawn Object Reference"))
  (set `self.hasFollowTarget` true)
  (`self.FollowTarget`))

(event `FollowTarget`
  (if (not (`self.isDead`))
    (if (`self.hasFollowTarget`)
      (if (`self.canMove`)
        (`|AIMoveTo` self (0.0 0.0 0.0) (`GameplayStatics.GetPlayerCharacter` 0) 40.0
          (:`OnSuccess`
            (if (`self.canAttack`)
              (set `self.canAttack` false)
              (set `self.canMove` false)
              (`self.TriggerCollision`)
              (bind _returnvalue (`self.PlayAnimMontage` "/Game/Resources/Monster/Animations/Attack1_Montage.Attack1_Montage"))
              (`KismetSystemLibrary.Delay` _returnvalue)
              (set `self.canAttack` true)
              (set `self.canMove` true)
              (`PrimitiveComponent.SetCollisionEnabled` (`self.Sphere`) "NoCollision"))))))
    (else
      (`KismetSystemLibrary.Delay` 2.5)
      (`self.K2_DestroyActor`))))

(event `TriggerCollision`
  (`KismetSystemLibrary.Delay` 0.5)
  (`PrimitiveComponent.SetCollisionEnabled` (`self.Sphere`) "QueryOnly"))

(event `self.Sphere.OnComponentBeginOverlap`
  (params (OverlappedComponent :type "PrimitiveComponent Object Reference") (OtherActor :type "Actor Object Reference") (OtherComp :type "PrimitiveComponent Object Reference") (OtherBodyIndex :type Integer) (bFromSweep :type Boolean) (SweepResult :type "HitResult Structure (by ref)"))
  (bind _asthird_person_character (cast `/Game/ThirdPersonCPP/Blueprints/ThirdPersonCharacter` OtherActor))
  (if (not (`DungeonCrawlerCharacter.m_isInvulnerable` _asthird_person_character))
    (`DungeonCrawlerCharacter.takeDamage` _asthird_person_character (`self.damage`))
    (`KismetSystemLibrary.PrintString` "Active HIT!!!")))

(fn `checkInvulnerability`
  (if (`self.isInvulnerable`)
    (if (>= (`self.invulnerabilityElapsed`) (`self.invulnerabilityTime`))
      (set `self.invulnerabilityElapsed` 0.0)
      (set `self.isInvulnerable` false)
      (else
        (set `self.invulnerabilityElapsed` (+ (`self.invulnerabilityElapsed`) (`GameplayStatics.GetWorldDeltaSeconds`)))))))

(fn `takeDamage`
  (params (damage :type "Float (double-precision)"))
  (if (and (not (`self.isInvulnerable`)) (not (`self.isDead`)))
    (bind _output_get (set `self.hp` (- (`self.hp`) (`local.damage`))))
    (set `self.hp` (`KismetMathLibrary.FClamp` _output_get 0.0 (`self.hpBase`)))
    (if (<= (`self.hp`) 0.0)
      (set `self.isDead` true)
      (`PrimitiveComponent.SetCollisionEnabled` (`self.CapsuleComponent`) "NoCollision")
      (bind _asthird_person_character (cast `/Game/ThirdPersonCPP/Blueprints/ThirdPersonCharacter` (`GameplayStatics.GetPlayerPawn` 0)))
      (`/Game/ThirdPersonCPP/Blueprints/ThirdPersonCharacter.addToKills` _asthird_person_character)
      (else
        (set `self.isInvulnerable` true)))))

(fn `UserConstructionScript`)