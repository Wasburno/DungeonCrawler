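; Spawner actor that periodically spawns BP_BasicEnemy at its own transform.
; While IsActive is set, Tick adds world delta time to an elapsed timer until it reaches the cooldown, then resets it and spawns.
; Spawning nudges the enemy clear of collisions and skips it if no free spot is found.
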(event `self.ReceiveTick`
  (params (DeltaSeconds :type "Float (single-precision)"))
  (if (`self.isActive`)
    (if (>= (`self.spawnElpased`) (`self.spawnCoolDown`))
      (set `self.spawnElpased` 0.0)
      (`|SpawnActorFromClass` "/Game/Blueprints/BP_BasicEnemy.BP_BasicEnemy_C" (`self.GetTransform`) "AdjustIfPossibleButDontSpawnIfColliding" "OverrideRootScale" null null)
      (else
        (set `self.spawnElpased` (+ (`self.spawnElpased`) (`GameplayStatics.GetWorldDeltaSeconds`)))))))

(fn `UserConstructionScript`)